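; AI-controlled player character with team-style tinting, sword combat and damage handling.
; MovePlayer forwards destinations to BP_AICon, while SetColor and the construction script tint dynamic body and head materials.
; AttackSword spins SwordStart on a timeline, line-tracing along the blade each update to damage other BP_PlayerChar hits by Strength.
; TakeDamage subtracts from MaxHealth, not Health, and asks BPGameManager to destroy the player at zero, naming the attacker.
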(event Custom|SetColor
  (params (Color :type String))
  (switch string Color
    (:Red
      (Variables|Default|SetColorVar "(R=0.583333,G=0.045573,B=0.045573,A=1.000000)"))
    (:Green
      (Variables|Default|SetColorVar "(R=0.104818,G=0.437500,B=0.104818,A=1.000000)"))
    (:Blue
      (Variables|Default|SetColorVar "(R=0.044922,G=0.044922,B=0.718750,A=1.000000)"))
    (:Purple
      (Variables|Default|SetColorVar "(R=0.061610,G=0.014106,B=0.104167,A=1.000000)"))
    (:Pink
      (Variables|Default|SetColorVar "(R=1.000000,G=0.109375,B=0.525000,A=1.000000)"))
    (:Yellow
      (Variables|Default|SetColorVar "(R=0.649154,G=0.661458,B=0.058567,A=1.000000)"))
    (:Orange
      (Variables|Default|SetColorVar "(R=0.673000,G=0.255682,B=0.000000,A=1.000000)")))
  (Rendering|Material|SetVectorParameterValue (Variables|Default|GetBodyDynMat) "BC_Tint" (Variables|Default|GetColorVar) :!class /Script/Engine.MaterialInstanceDynamic))

(event Custom|AttackSword
  (bind _newtrack_0 (Timeline|Timeline PlayFromStart)
    (:Update
      (Transformation|SetRelativeRotation (Variables|Default|GetSwordStart) (Math|Rotator|Lerp(Rotator) "0, 0, 0" "0.000000,-360.000000,0.000000" _newtrack_0) false false)
      (bind (_outhit _returnvalue) (Collision|LineTraceByChannel (Transformation|GetWorldLocation (Variables|Default|GetSwordStart)) (Transformation|GetWorldLocation (Variables|Default|GetSwordEnd)) "TraceTypeQuery1" false 0 "None"))
      (if _returnvalue
        (bind _asbp_player_char (Utilities|Casting|CastToBP_PlayerChar (.HitActor (Collision|BreakHitResult _outhit))))
        (CallFunction|TakeDamage _asbp_player_char (Variables|Default|GetStrength) (Variables|Default|GetOwningPlayerName))))))

(event Custom|TakeDamage
  (params (Damage :type Float%20%28single-precision%29) (AttackedBy :type String))
  (Variables|Default|SetAttackedBy AttackedBy)
  (bind _output_get (Variables|Default|SetMaxHealth (- (Variables|Default|GetMaxHealth) Damage)))
  (Development|PrintString (Utilities|String|ToString(Float) _output_get))
  (if (<= _output_get 0.0)
    (Default|DestroyPlayer (Variables|Default|GetBP_GameManager) self (Variables|Default|GetOwningPlayerName) (Variables|Default|GetAttackedBy))))

(event EventBeginPlay
  (Variables|Default|SetHealth (Variables|Default|GetMaxHealth))
  (bind _asbp_aicon (Utilities|Casting|CastToBP_AICon (AI|GetAIController self)))
  (Variables|Default|SetAICon _asbp_aicon)
  (Development|PrintString (Variables|Default|GetOwningPlayerName)))

(event Collision|EventActorBeginOverlap
  (params (OtherActor :type Actor%20Object%20Reference)))

(event EventTick
  (params (DeltaSeconds :type Float%20%28single-precision%29))
  (Transformation|SetWorldRotation (Variables|Default|GetArrow1) "0, 0, 0" false false))

(fn ConstructionScript
  (bind _returnvalue (Rendering|Material|CreateDynamicMaterialInstance (Variables|Default|GetCylinder) 0 0 "None" :!class /Script/Engine.PrimitiveComponent))
  (Variables|Default|SetBodyDynMat _returnvalue)
  (bind _returnvalue_2 (Rendering|Material|CreateDynamicMaterialInstance (Variables|Default|GetSphere) 0 0 "None" :!class /Script/Engine.PrimitiveComponent))
  (Variables|Default|SetHeadDynMat _returnvalue_2)
  (Rendering|Material|SetVectorParameterValue (Variables|Default|GetBodyDynMat) "BC_Tint" (Variables|Default|GetColorVar) :!class /Script/Engine.MaterialInstanceDynamic))

(fn MovePlayer
  (params (Dest :type Vector%20%28by%20ref%29))
  (bind _success (Default|MovePlayertoLocation (Variables|Default|GetAICon) Dest))
  (return _success))