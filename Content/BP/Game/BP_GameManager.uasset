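; Game manager for a Twitch chat-driven game where viewers spawn and control their own characters.
; On BeginPlay it optionally logs into Twitch, opens a chat feed and registers join, move, setcolor and attack commands.
; UserInfoArray maps chatters to pawns and scores, crediting kills and updating a scoreboard, whose creation is disconnected.
; Moves fall back to trace-based navigable points; separate Twitch SDK auth and prediction events have no active caller here.
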(event Custom|SetUpTwitch
  ;[1 1 1] Set Up Twitch
  (if (Variables|MainData|GetturnOnTwitch?)
    (bind _credentials (|PerformTwitchLogin)
      (:OnSuccess
        (Development|PrintString "Twitch Log in succeeded")
        (bind _twitchchat (|RequestFeed (delegate Custom|OnChatEntered) (delegate Custom|OnCheerEvent) _credentials (.Username (Utilities|Struct|BreakTwitchLoginCredentials _credentials)))
          (:OnSuccessfulLogin
            (Development|PrintString (.Username (Utilities|Struct|BreakTwitchLoginCredentials _credentials)))
            (Variables|MainData|SetTwitch%20Chat _twitchchat)
            (CallFunction|SetAllTwitchCommands))))
      (:OnFail
        (Development|PrintString "Twitch Log In Failed")))))

(event Custom|OnChatEntered
  (params (TwitchMessage :type Twitch%20Message%20Structure))
  ;[1 1 1] Set Up Twitch
)

(event Custom|OnCheerEvent
  (params (TwitchCheer :type Twitch%20Cheer%20Structure))
  ;[1 1 1] Set Up Twitch
)

(event Custom|SetAllTwitchCommands
  (Utilities|FlowControl|Sequence
    (:then_0
      (|JoinCommand))
    (:then_1
      (|MoveCommand))
    (:then_2
      (|SetColorCommand))
    (:then_3
      (|AttackCommand))))

(event Custom|DestroyPlayer
  (params (PlayerChar :type BP%20Player%20Char%20Object%20Reference) (PlayerName :type String) (AttackingPlayerName :type String))
  (|DestroyPlayerGraph PlayerChar PlayerName AttackingPlayerName))

(event Custom|UpdateScoreUI
  ;[1 1 1] Set Up Twitch
)

(event Custom|Start%20a%20prediction
  ;[0.06863 0.5729 0.08891] Initiate Prediction with Possible Choices.
  ; Save Prediction ID and Broadcaster ID Variables.
  (bind (_result _error) (|Prediction "Did this prediction work?" (Variables|Default|GetPredictionOutcomes) 30)
    (:Done
      (Variables|Default|SetPredictionID (.id _result))
      (Variables|Default|SetBroadcasterID (.broadcasterid _result))
      ;[0.1715 0.06117 0.2865] Check for updates on prediction.
      ; When time is up, Set Results as array variable.
      (bind (_result_2 _error_2) (|WaitforPredictionUpdate (Variables|Default|GetPredictionID) :!label _label)
        (:Done
          (switch Utilities|FlowControl|Switch|SwitchonFTwitchSDKPredictionStatus (.status _result_2)
            (:Active
              (Development|PrintString "Active" true true "(R=0.000000,G=0.660000,B=1.000000,A=1.000000)" 3e+01)
              (goto _label))
            (:Locked
              (Variables|Default|SetPredictionResults (.outcomes _result_2))
              ;[0.4128 0.4844 0.02612] Trigger whatever event is being predicted
              ; Set Winning Result Text...
              ; After results call next section.
              (Utilities|FlowControl|Delay 0.2)
              (Variables|Default|SetWinningOutcomeText "")
              ;[0.1277 0.2608 0.625] Loop through winning results, find
              (bind _array_element (Utilities|Array|ForEachLoopwithBreak (Variables|Default|GetPredictionResults) :!label _label_2)
                (:LoopBody
                  (if (Utilities|Enum|Equal(Enum) (.Title (Utilities|Struct|BreakTwitchSDKPredictionOutcome _array_element)) (Variables|Default|GetWinningOutcomeText))
                    (Variables|Default|SetWinningResult _array_element)
                    (goto _label_2 Break)))
                (:Completed
                  ;[0.4269 0.2537 0.625] Finalize Prediction Winnings.
                  ; Give Out Rewards To Winners.
                  (bind (_result_3 _error_3) (|EndPrediction (Variables|Default|GetBroadcasterID) (Variables|Default|GetPredictionID) "Resolved" (.Id (Utilities|Struct|BreakTwitchSDKPredictionOutcome (Variables|Default|GetWinningResult))))
                    (:Done
                      (switch Utilities|FlowControl|Switch|SwitchonFTwitchSDKPredictionStatus (.status _result_3)
                        (:Active
                          ;[0.2031 0.02433 0.02433] Cancel Prediction.
                          (bind _error_4 (|EndPrediction (Variables|Default|GetBroadcasterID) (Variables|Default|GetPredictionID) "Canceled" :!label _label_3)
                            (:Done
                              _)
                            (:Error
                              ;[0.5417 0 0] Print Errors if anything fails during prediction
                              ; Then cancels the prediction and unsubscribes.
                              (Development|PrintString _error_4 true true "(R=0.000000,G=0.660000,B=1.000000,A=1.000000)" 3e+01))))
                        (:Locked
                          (goto _label_3))
                        (:Resolved
                          _)
                        (:Canceled
                          _)))
                    (:Error
                      (Development|PrintString _error_3 true true "(R=0.000000,G=0.660000,B=1.000000,A=1.000000)" 3e+01)
                      (goto _label_3)))
                  ;[0.2083 0.2083 0.2083] Unsubscribe from prediction to prevent unneccessary network traffic
                  (|UnsubscribefromPrediction (Variables|Default|GetPredictionID) :!label _label_4))))
            (:Resolved
              (goto _label_3))
            (:Canceled
              (goto _label_4))))
        (:Error
          (Development|PrintString _error_2 true true "(R=0.000000,G=0.660000,B=1.000000,A=1.000000)" 3e+01)
          (goto _label_3))))
    (:Error
      (Development|PrintString _error)
      (goto _label_3))))

(event Custom|CallCancelPrediction
  ;[0.2031 0.02433 0.02433] Cancel Prediction.
  (bind _error (|EndPrediction (Variables|Default|GetBroadcasterID) (Variables|Default|GetPredictionID) "Canceled")
    (:Done
      _)
    (:Error
      ;[0.5417 0 0] Print Errors if anything fails during prediction
      ; Then cancels the prediction and unsubscribes.
      (Development|PrintString _error true true "(R=0.000000,G=0.660000,B=1.000000,A=1.000000)" 3e+01)))
  ;[0.2083 0.2083 0.2083] Unsubscribe from prediction to prevent unneccessary network traffic
  (|UnsubscribefromPrediction (Variables|Default|GetPredictionID)))

(event Custom|Setup%20Twitch%20SDK
  ;[0.0396 0.4323 0.1104] Setup Twitch Initial Login
  ;;[0.1639 0.1896 0.7083] Check current login state
  (bind _result (|GetAuthState)
    (:Done
      (if (Utilities|Enum|Equal(Enum) (.Status (Utilities|Struct|BreakTwitchSDKAuthState _result)) "LoggedOut")
        ;;[1 0.3958 0.3958] Get URI And Authorization Code
        ;;  To Connect To Twitch
        (bind (_result_2 _error) (|GetAuthenticationInfo (Class|TwitchSDKBPLibrary|BuildOAuthScopes (Utilities|Array|MakeArray "ChannelManagePolls" "ChannelManagePredictions" "ChannelManageBroadcast" "ChannelManageRedemptions" "ChannelReadHype_Train" "ClipsEdit" "UserReadSubscriptions" "BitsRead")) :!label _label)
          (:Done
            (Development|PrintString (Utilities|String|ToString(Text) (Utilities|Text|FormatText "The uri is {uri}  
The user code is {usercode}" (.Uri (Utilities|Struct|BreakTwitchSDKAuthenticationInfo _result_2)) (.UserCode (Utilities|Struct|BreakTwitchSDKAuthenticationInfo _result_2)))) true true "(R=0.000000,G=0.660000,B=1.000000,A=1.000000)" 3e+01)
            ;;[0.2351 0.6257 1] Check if can connect to twitch
            ;; Load URL in browser for authorization.
            (Variables|Default|SetOauth (Utilities|String|Append (.Uri (Utilities|Struct|BreakTwitchSDKAuthenticationInfo _result_2)) (.UserCode (Utilities|Struct|BreakTwitchSDKAuthenticationInfo _result_2))))
            (bind _returnvalue (Class|KismetSystemLibrary|CanLaunchURL (Utilities|String|Append (.Uri (Utilities|Struct|BreakTwitchSDKAuthenticationInfo _result_2)) (.UserCode (Utilities|Struct|BreakTwitchSDKAuthenticationInfo _result_2)))))
            (if _returnvalue
              (Utilities|FlowControl|Sequence
                (:then_0
                  (Utilities|FlowControl|DoOnce false
                    (:Completed
                      (Utilities|Platform|LaunchURL (Utilities|String|Append (.Uri (Utilities|Struct|BreakTwitchSDKAuthenticationInfo _result_2)) (.UserCode (Utilities|Struct|BreakTwitchSDKAuthenticationInfo _result_2)))))))
                (:then_1
                  ;;[0.2267 1 0.1927] After Failed URL Launch or after launching URL
                  ;; Wait then Call Set Up Twitch Again to check for successful login.
                  (Utilities|FlowControl|Delay 1.0 :!label _label_2)
                  (CallFunction|SetUpTwitch)))
              (else
                (goto _label_2))))
          (:Error
            ;;[1 0.01562 0.01562] Log Error if Twitch Authentication Fails To Load Info
            (Development|PrintString (Utilities|String|Append "Twitch Error: " _error) true true "(R=0.000000,G=0.660000,B=1.000000,A=1.000000)" 2e+01)))
        (else
          (if (Utilities|Enum|Equal(Enum) (.Status (Utilities|Struct|BreakTwitchSDKAuthState _result)) "Loading")
            _
            (else
              _))
          (if (Utilities|Enum|Equal(Enum) (.Status (Utilities|Struct|BreakTwitchSDKAuthState _result)) "LoggedIn")
            ;;[0.05208 1 1] If Logged In, Call Start Prediction
            (Development|PrintString "Already Logged In" true true "(R=0.000000,G=0.660000,B=1.000000,A=1.000000)" 3e+01)
            (else
              (goto _label))))))))

(event EventBeginPlay
  ;[1 1 1] Begin Play / Call Setup Twitch
  (CallFunction|SetUpTwitch))

(fn ConstructionScript)

(event Custom|JoinPlayer
  (params (Parameters :type Array%20of%20Strings) (Sender :type Twitch%20Message%20Author%20Structure))
  (Variables|JoinData|SetCurrJoinSenderInfo Sender)
  (bind _array_element (Utilities|Array|ForEachLoopwithBreak (Variables|MainData|GetUserInfoArray) :!label _label)
    (:LoopBody
      (if (Utilities|Enum|Equal(Enum) (.PlayerName (Utilities|Struct|BreakS_UserInfo _array_element)) (.Name (Utilities|Struct|BreakTwitchMessageAuthor (Variables|JoinData|GetCurrJoinSenderInfo))))
        (Variables|JoinData|SetJoinPlayerFound? true)
        (goto _label Break)
        (else
          (Variables|JoinData|SetJoinPlayerFound? false))))
    (:Completed
      (if (Variables|JoinData|GetJoinPlayerFound?)
        (Class|TwitchPluginBPLibrary|SendTwitchMessage (Variables|MainData|GetTwitch%20Chat) (Utilities|String|Append "@" (.Name (Utilities|Struct|BreakTwitchMessageAuthor (Variables|JoinData|GetCurrJoinSenderInfo))) " You already have a player in game, type !help to see commands."))
        (else
          (bind _randomlocation (Class|NavigationSystemV1|GetRandomLocationinNavigableRadius (Math|Vector|MakeVector 0.0 0.0 0.0) 5e+02 0 0))
          (bind _returnvalue (Game|SpawnActorfromClass "/Game/BP/Character/BP_PlayerChar.BP_PlayerChar_C" (Math|Transform|MakeTransform _randomlocation "0, 0, 0" "2.000000,2.000000,2.000000") "Undefined" "MultiplyWithRoot" 0 (Variables|JoinData|GetJoinColorVar) self (.Name (Utilities|Struct|BreakTwitchMessageAuthor (Variables|JoinData|GetCurrJoinSenderInfo))) 0))
          (Rendering|Components|TextRender|SetText (Variables|/Game/BP/Character/BP_PlayerChar.BP_PlayerChar_C|GetTextRender _returnvalue) (Utilities|Text|ToText(String) (.Name (Utilities|Struct|BreakTwitchMessageAuthor (Variables|JoinData|GetCurrJoinSenderInfo)))))
          (Utilities|Array|AddUnique (Variables|MainData|GetUserInfoArray) (Utilities|Struct|MakeS_UserInfo (.Name (Utilities|Struct|BreakTwitchMessageAuthor (Variables|JoinData|GetCurrJoinSenderInfo))) _returnvalue 0))
          (Default|SetValues (Variables|Default|GetW_Scoreboard) (Variables|MainData|GetUserInfoArray)))))))

(event Custom|AttackPlayer
  (params (Parameters :type Array%20of%20Strings) (Sender :type Twitch%20Message%20Author%20Structure))
  (bind _output_get (Variables|Default|SetCurAttackSender Sender))
  (bind (_array_element _array_index) (Utilities|Array|ForEachLoopwithBreak (Variables|MainData|GetUserInfoArray) :!label _label)
    (:LoopBody
      (if (Utilities|Enum|Equal(Enum) (.PlayerName (Utilities|Struct|BreakS_UserInfo _array_element)) (.Name (Utilities|Struct|BreakTwitchMessageAuthor _output_get)))
        (Variables|Default|SetAttackPlayerFound? true)
        (Variables|Default|SetCurrAttackPlayerInd _array_index)
        (goto _label Break)
        (else
          (Variables|Default|SetAttackPlayerFound? false))))
    (:Completed
      (if (Variables|Default|GetAttackPlayerFound?)
        (Default|AttackSword (.PlayerPawn (Utilities|Struct|BreakS_UserInfo (Utilities|Array|Get(acopy) (Variables|MainData|GetUserInfoArray) (Variables|Default|GetCurrAttackPlayerInd)))))
        (else
          (Class|TwitchPluginBPLibrary|SendTwitchMessage (Variables|MainData|GetTwitch%20Chat) (Utilities|String|Append "@" (.Name (Utilities|Struct|BreakTwitchMessageAuthor _output_get)) " You do not have a player in game, type join to create a new player.")))))))

(event Custom|MovePlayer
  (params (Parameters :type Array%20of%20Strings) (Sender :type Twitch%20Message%20Author%20Structure))
  (Variables|MoveData|SetCurrMoveParams Parameters)
  (bind _output_get (Variables|MoveData|SetCurrMoveSenderInfo Sender))
  (bind (_array_element _array_index) (Utilities|Array|ForEachLoopwithBreak (Variables|MainData|GetUserInfoArray) :!label _label)
    (:LoopBody
      (if (Utilities|Enum|Equal(Enum) (.PlayerName (Utilities|Struct|BreakS_UserInfo _array_element)) (.Name (Utilities|Struct|BreakTwitchMessageAuthor _output_get)))
        (Variables|MoveData|SetMovePlayerFound? true)
        (Variables|MoveData|SetcurrMovePlayerInd _array_index)
        (goto _label Break)
        (else
          (Variables|MoveData|SetMovePlayerFound? false))))
    (:Completed
      (if (Variables|MoveData|GetMovePlayerFound?)
        (switch string (Utilities|Array|Get(acopy) (Variables|MoveData|GetCurrMoveParams))
          (:Default
            (bind _returnvalue (Transformation|SetActorRotation (.PlayerPawn (Utilities|Struct|BreakS_UserInfo (Utilities|Array|Get(acopy) (Variables|MainData|GetUserInfoArray) (Variables|MoveData|GetcurrMovePlayerInd)))) (Math|Rotator|MakeRotator 0.0 0.0 (Math|Conversions|ToFloat(Integer) (Utilities|Array|Get(acopy) (Variables|MoveData|GetCurrMoveParams))))))
            (if _returnvalue
              (bind _success (Default|MovePlayer (.PlayerPawn (Utilities|Struct|BreakS_UserInfo (Utilities|Array|Get(acopy) (Variables|MainData|GetUserInfoArray) (Variables|MoveData|GetcurrMovePlayerInd)))) (+ (Transformation|GetActorLocation (.PlayerPawn (Utilities|Struct|BreakS_UserInfo (Utilities|Array|Get(acopy) (Variables|MainData|GetUserInfoArray) (Variables|MoveData|GetcurrMovePlayerInd))))) (* (Transformation|GetActorForwardVector (.PlayerPawn (Utilities|Struct|BreakS_UserInfo (Utilities|Array|Get(acopy) (Variables|MainData|GetUserInfoArray) (Variables|MoveData|GetcurrMovePlayerInd))))) (* (Math|Conversions|ToFloat(Integer) (Utilities|Array|Get(acopy) (Variables|MoveData|GetCurrMoveParams) 1)) 1e+01)))))
              (if _success
                (Development|PrintString "Nav Successful at point 1")
                (else
                  (bind _outhit (Collision|LineTraceByChannel (+ (Transformation|GetActorLocation (.PlayerPawn (Utilities|Struct|BreakS_UserInfo (Utilities|Array|Get(acopy) (Variables|MainData|GetUserInfoArray) (Variables|MoveData|GetcurrMovePlayerInd))))) "0.000000,0.000000,50.000000") (+ (+ (Transformation|GetActorLocation (.PlayerPawn (Utilities|Struct|BreakS_UserInfo (Utilities|Array|Get(acopy) (Variables|MainData|GetUserInfoArray) (Variables|MoveData|GetcurrMovePlayerInd))))) (* (Transformation|GetActorForwardVector (.PlayerPawn (Utilities|Struct|BreakS_UserInfo (Utilities|Array|Get(acopy) (Variables|MainData|GetUserInfoArray) (Variables|MoveData|GetcurrMovePlayerInd))))) (* (Math|Conversions|ToFloat(Integer) (Utilities|Array|Get(acopy) (Variables|MoveData|GetCurrMoveParams) 1)) 1e+01))) "0.000000,0.000000,50.000000") "TraceTypeQuery1" false (Utilities|Array|MakeArray (.PlayerPawn (Utilities|Struct|BreakS_UserInfo (Utilities|Array|Get(acopy) (Variables|MainData|GetUserInfoArray) (Variables|MoveData|GetcurrMovePlayerInd))))) "ForDuration" true "(R=1.000000,G=0.000000,B=0.000000,A=1.000000)" "(R=0.000000,G=1.000000,B=0.000000,A=1.000000)" 1e+02))
                  (bind (_randomlocation _returnvalue_2) (Class|NavigationSystemV1|GetRandomLocationinNavigableRadius (.Location (Collision|BreakHitResult _outhit)) 2.5e+02 0 0))
                  (if _returnvalue_2
                    (bind _success_2 (Default|MovePlayer (.PlayerPawn (Utilities|Struct|BreakS_UserInfo (Utilities|Array|Get(acopy) (Variables|MainData|GetUserInfoArray) (Variables|MoveData|GetcurrMovePlayerInd)))) _randomlocation))
                    (if _success_2
                      (Development|PrintString "Nav Successful at point 2")
                      (else
                        (Development|PrintString "Nav Failed at point 2"))))))
              (else
                (Class|TwitchPluginBPLibrary|SendTwitchMessage (Variables|MainData|GetTwitch%20Chat) (Utilities|String|Append "@" (.Name (Utilities|Struct|BreakTwitchMessageAuthor (Variables|MoveData|GetCurrMoveSenderInfo))) " " (Utilities|Array|Get(acopy) (Variables|MoveData|GetCurrMoveParams)) " Is not a valid number")))))
          (:up
            (Variables|MoveData|SetMoveDir "1.000000,0.000000,0.000000")
            (bind _success_3 (Default|MovePlayer (.PlayerPawn (Utilities|Struct|BreakS_UserInfo (Utilities|Array|Get(acopy) (Variables|MainData|GetUserInfoArray) (Variables|MoveData|GetcurrMovePlayerInd)))) (+ (Transformation|GetActorLocation (.PlayerPawn (Utilities|Struct|BreakS_UserInfo (Utilities|Array|Get(acopy) (Variables|MainData|GetUserInfoArray) (Variables|MoveData|GetcurrMovePlayerInd))))) (* (Variables|MoveData|GetMoveDir) (* (Math|Conversions|ToFloat(Integer) (Utilities|Array|Get(acopy) (Variables|MoveData|GetCurrMoveParams) 1)) 1e+01))) :!label _label_2))
            (if _success_3
              (Development|PrintString "Nav Successful at point 1")
              (else
                (bind _outhit_2 (Collision|LineTraceByChannel (+ (Transformation|GetActorLocation (.PlayerPawn (Utilities|Struct|BreakS_UserInfo (Utilities|Array|Get(acopy) (Variables|MainData|GetUserInfoArray) (Variables|MoveData|GetcurrMovePlayerInd))))) "0.000000,0.000000,50.000000") (+ (+ (Transformation|GetActorLocation (.PlayerPawn (Utilities|Struct|BreakS_UserInfo (Utilities|Array|Get(acopy) (Variables|MainData|GetUserInfoArray) (Variables|MoveData|GetcurrMovePlayerInd))))) (* (Variables|MoveData|GetMoveDir) (* (Math|Conversions|ToFloat(Integer) (Utilities|Array|Get(acopy) (Variables|MoveData|GetCurrMoveParams) 1)) 1e+01))) "0.000000,0.000000,50.000000") "TraceTypeQuery1" false (Utilities|Array|MakeArray (.PlayerPawn (Utilities|Struct|BreakS_UserInfo (Utilities|Array|Get(acopy) (Variables|MainData|GetUserInfoArray) (Variables|MoveData|GetcurrMovePlayerInd))))) "ForDuration" true "(R=1.000000,G=0.000000,B=0.000000,A=1.000000)" "(R=0.000000,G=1.000000,B=0.000000,A=1.000000)" 1e+02))
                (bind (_randomlocation_2 _returnvalue_3) (Class|NavigationSystemV1|GetRandomLocationinNavigableRadius (.Location (Collision|BreakHitResult _outhit_2)) 2.5e+02 0 0))
                (if _returnvalue_3
                  (bind _success_4 (Default|MovePlayer (.PlayerPawn (Utilities|Struct|BreakS_UserInfo (Utilities|Array|Get(acopy) (Variables|MainData|GetUserInfoArray) (Variables|MoveData|GetcurrMovePlayerInd)))) _randomlocation_2))
                  (if _success_4
                    (Development|PrintString "Nav Successful at point 2")
                    (else
                      (Development|PrintString "Nav Failed at point 2")))))))
          (:left
            (Variables|MoveData|SetMoveDir "0.000000,-1.000000,0.000000")
            (goto _label_2))
          (:right
            (Variables|MoveData|SetMoveDir "0.000000,1.000000,0.000000")
            (goto _label_2))
          (:down
            (Variables|MoveData|SetMoveDir "-1.000000,0.000000,0.000000")
            (goto _label_2))
          (:upright
            (Variables|MoveData|SetMoveDir "0.500000,0.500000,0.000000" :!label _label_3)
            (goto _label_2))
          (:ur
            (goto _label_3))
          (:rightup
            (goto _label_3))
          (:ru
            (goto _label_3))
          (:leftup
            (Variables|MoveData|SetMoveDir "0.500000,-0.500000,0.000000" :!label _label_4)
            (goto _label_2))
          (:lu
            (goto _label_4))
          (:upleft
            (goto _label_4))
          (:ul
            (goto _label_4))
          (:downleft
            (Variables|MoveData|SetMoveDir "-0.500000,-0.500000,0.000000" :!label _label_5)
            (goto _label_2))
          (:dl
            (goto _label_5))
          (:leftdown
            (goto _label_5))
          (:ld
            (goto _label_5))
          (:rightdown
            (Variables|MoveData|SetMoveDir "-0.500000,0.500000,0.000000" :!label _label_6)
            (goto _label_2))
          (:rd
            (goto _label_6))
          (:downright
            (goto _label_6))
          (:dr
            (goto _label_6)))
        (else
          (Class|TwitchPluginBPLibrary|SendTwitchMessage (Variables|MainData|GetTwitch%20Chat) (Utilities|String|Append "@" (.Name (Utilities|Struct|BreakTwitchMessageAuthor _output_get)) " You do not have a player in game, type join to create a new player.")))))))

(event Custom|SetColorPlayer
  (params (Parameters :type Array%20of%20Strings) (Sender :type Twitch%20Message%20Author%20Structure))
  (Variables|SetColorData|SetCurSetColorParams Parameters)
  (bind _output_get (Variables|SetColorData|SetCurrSetColorSenderInfo Sender))
  (bind (_array_element _array_index) (Utilities|Array|ForEachLoopwithBreak (Variables|MainData|GetUserInfoArray) :!label _label)
    (:LoopBody
      (if (Utilities|Enum|Equal(Enum) (.PlayerName (Utilities|Struct|BreakS_UserInfo _array_element)) (.Name (Utilities|Struct|BreakTwitchMessageAuthor _output_get)))
        (Variables|SetColorData|SetSetColorPlayerFound? true)
        (Variables|SetColorData|SetcurrSetColorPlayerInd _array_index)
        (goto _label Break)
        (else
          (Variables|SetColorData|SetSetColorPlayerFound? false))))
    (:Completed
      (if (Variables|SetColorData|GetSetColorPlayerFound?)
        (Default|SetColor (.PlayerPawn (Utilities|Struct|BreakS_UserInfo (Utilities|Array|Get(acopy) (Variables|MainData|GetUserInfoArray) (Variables|SetColorData|GetcurrSetColorPlayerInd)))) (Utilities|Array|Get(acopy) (Variables|SetColorData|GetCurSetColorParams)))
        (else
          (Class|TwitchPluginBPLibrary|SendTwitchMessage (Variables|MainData|GetTwitch%20Chat) (Utilities|String|Append "@" (.Name (Utilities|Struct|BreakTwitchMessageAuthor _output_get)) " You do not have a player in game, type join to create a new player.")))))))