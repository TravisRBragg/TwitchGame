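; BP_Planter is a planter actor for growing cannabis through plant, water and harvest events, registering itself with the Twitch game instance on BeginPlay.
; One CropState enum combines growth stage and wet/dry condition, so watering a seeded or growing crop starts a fixed delay that advances it to the next dry stage until flowering.
; Stages swap the crop mesh, a dynamic dirt material shows wetness, and construction randomises crop yaw.
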(event Custom|CallStageTimeline
  (Utilities|FlowControl|Delay 5.0)
  (switch Utilities|FlowControl|Switch|SwitchonE_CropState (Variables|Default|GetCropState)
    (:NewEnumerator3
      (CallFunction|SetCropMesh "/Game/Twitch/Art/Mesh/Crops/Cannabis/Merged/SM_Cannabis_Sapling.SM_Cannabis_Sapling")
      (Variables|Default|SetCropState "NewEnumerator10"))
    (:NewEnumerator11
      (CallFunction|SetCropMesh "/Game/Twitch/Art/Mesh/Crops/Cannabis/Merged/SM_Cannabis_Half.SM_Cannabis_Half")
      (Variables|Default|SetCropState "NewEnumerator4"))
    (:NewEnumerator5
      (CallFunction|SetCropMesh "/Game/Twitch/Art/Mesh/Crops/Cannabis/Merged/SM_Cannabis_Full_NoFlower.SM_Cannabis_Full_NoFlower")
      (Variables|Default|SetCropState "NewEnumerator6"))
    (:NewEnumerator7
      (CallFunction|SetCropMesh "/Game/Twitch/Art/Mesh/Crops/Cannabis/Merged/SM_Cannabis_Full.SM_Cannabis_Full")
      (Variables|Default|SetCropState "NewEnumerator8")))
  (CallFunction|SetIsWatered)
  (Variables|Default|SetisWatered false))

(event EventBeginPlay
  (|CallParentFunction)
  (Default|AddPlanterRef (Variables|Default|GetTwitch_Game_Instance) self))

(event Collision|EventActorBeginOverlap
  (params (OtherActor :type Actor%20Object%20Reference))
  (|CallParentFunction OtherActor) ; This node is disabled and will not be called.\nDrag off pins to build functionality.
)

(event EventTick
  (params (DeltaSeconds :type Float%20%28single-precision%29))
  (|CallParentFunction DeltaSeconds) ; This node is disabled and will not be called.\nDrag off pins to build functionality.
)

(event EventPlantSeed
  (CallFunction|SetCropMesh "/Game/Twitch/Art/Mesh/Crops/Cannabis/Merged/SM_Cannabis_Seeds.SM_Cannabis_Seeds")
  (switch Utilities|FlowControl|Switch|SwitchonE_CropState (Variables|Default|GetCropState)
    (:NewEnumerator0
      (Variables|Default|SetCropState "NewEnumerator1"))
    (:NewEnumerator2
      (Variables|Default|SetCropState "NewEnumerator3")
      (CallFunction|CallStageTimeline)))
  (Variables|Default|SetisBeingInteractedWith false))

(event EventWaterCrop
  (switch Utilities|FlowControl|Switch|SwitchonE_CropState (Variables|Default|GetCropState)
    (:NewEnumerator0
      (Variables|Default|SetCropState "NewEnumerator2"))
    (:NewEnumerator1
      (Variables|Default|SetCropState "NewEnumerator3"))
    (:NewEnumerator10
      (Variables|Default|SetCropState "NewEnumerator11"))
    (:NewEnumerator4
      (Variables|Default|SetCropState "NewEnumerator5"))
    (:NewEnumerator6
      (Variables|Default|SetCropState "NewEnumerator7")))
  (CallFunction|SetIsWatered)
  (CallFunction|CallStageTimeline)
  (Variables|Default|SetisBeingInteractedWith false)
  (Variables|Default|SetisWatered true))

(event EventHarvestPlant
  (switch Utilities|FlowControl|Switch|SwitchonE_CropState (Variables|Default|GetCropState)
    (:NewEnumerator8
      _)
    (:NewEnumerator9
      _))
  (Variables|Default|SetCropState "NewEnumerator0")
  (CallFunction|SetCropMesh)
  (CallFunction|SetIsWatered)
  (Variables|Default|SetisBeingInteractedWith false)
  (Variables|Default|SetisWatered false))

(event EventSetIsInteracted
  (params (isBeingInteractedWith :type Boolean))
  (Variables|Default|SetisBeingInteractedWith isBeingInteractedWith))

(fn ConstructionScript
  (|CallParentFunction)
  (Transformation|SetRelativeRotation (Variables|Default|GetCrop) (Math|Rotator|MakeRotator 0.0 0.0 (Math|Random|RandomFloatinRange 0.0 3.6e+02)) false false)
  (bind _returnvalue (Rendering|Material|CreateDynamicMaterialInstance (Variables|Default|GetStaticMesh) 0 0 "None" :!class /Script/Engine.PrimitiveComponent))
  (Variables|Default|SetDirt_Dyn_Mat _returnvalue))

(fn SetCropMesh
  (params (NewMesh :type Static%20Mesh%20Object%20Reference))
  (Components|StaticMesh|SetStaticMesh (Variables|Default|GetCrop) NewMesh))

(fn SetIsWatered
  (bind _dirt_dyn_mat (Variables|Default|GetDirt_Dyn_Mat))
  (switch Utilities|FlowControl|Switch|SwitchonE_CropState (Variables|Default|GetCropState)
    (:NewEnumerator0
      (Rendering|Material|SetScalarParameterValue _dirt_dyn_mat "Wetness" 0.0 :!class /Script/Engine.MaterialInstanceDynamic :!label _label))
    (:NewEnumerator2
      (Rendering|Material|SetScalarParameterValue _dirt_dyn_mat "Wetness" 1.0 :!class /Script/Engine.MaterialInstanceDynamic :!label _label_2))
    (:NewEnumerator1
      (goto _label))
    (:NewEnumerator3
      (goto _label_2))
    (:NewEnumerator10
      (goto _label))
    (:NewEnumerator11
      (goto _label_2))
    (:NewEnumerator4
      (goto _label))
    (:NewEnumerator5
      (goto _label_2))
    (:NewEnumerator6
      (goto _label))
    (:NewEnumerator7
      (goto _label_2))
    (:NewEnumerator8
      (goto _label))
    (:NewEnumerator9
      (goto _label_2))))

(fn GetCurrentState
  (return (Variables|Default|GetCropState)))