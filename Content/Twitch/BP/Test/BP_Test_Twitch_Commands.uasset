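; BP_Test_Twitch_Commands is a debug actor for manually testing Twitch prediction and poll calls through BP_GM_Twitch.
; On BeginPlay it enables input from player controller 0 and caches the game mode cast to BP_GM_Twitch.
; Numpad keys call that game mode with hardcoded test data to create, resolve or cancel a prediction, or to create a poll.
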(event EventBeginPlay
  (Input|EnableInput (Game|GetPlayerController 0))
  (bind _asbp_gm_twitch (Utilities|Casting|CastToBP_GM_Twitch (Game|GetGameMode)))
  (Variables|Default|SetAs%20BP%20GM%20Twitch _asbp_gm_twitch))

(event Collision|EventActorBeginOverlap
  (params (OtherActor :type Actor%20Object%20Reference)))

(event EventTick
  (params (DeltaSeconds :type Float%20%28single-precision%29)))

(event Input|KeyboardEvents|NumPadOne
  (params (Key :type Key%20Structure :default "None"))
  (:Pressed
    (Default|CallCreatePrediction (Variables|Default|GetAs%20BP%20GM%20Twitch) "Did this shit work properly?" (Utilities|Array|MakeArray "Yes" "No" "Why would it" "Fail" "....") 30)))

(event Input|KeyboardEvents|NumPadFive
  (params (Key :type Key%20Structure :default "None"))
  (:Pressed
    (Default|CallCreatePoll (Variables|Default|GetAs%20BP%20GM%20Twitch) "Do you guys like boobs?" (Utilities|Array|MakeArray "Duh" "No" "Gross" "Whats that") 20 false 0 false)))

(event Input|KeyboardEvents|NumPadTwo
  (params (Key :type Key%20Structure :default "None"))
  (:Pressed
    (Default|CallResolvePrediction (Variables|Default|GetAs%20BP%20GM%20Twitch) "Yes")))

(event Input|KeyboardEvents|NumPadThree
  (params (Key :type Key%20Structure :default "None"))
  (:Pressed
    (Default|CallResolvePrediction (Variables|Default|GetAs%20BP%20GM%20Twitch) "No")))

(event Input|KeyboardEvents|NumPadFour
  (params (Key :type Key%20Structure :default "None"))
  (:Pressed
    (Default|CallCancelPrediction (Variables|Default|GetAs%20BP%20GM%20Twitch))))

(fn ConstructionScript)