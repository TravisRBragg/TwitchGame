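; Game instance that connects the game to Twitch and turns chatters into in-game characters.
; On init it retries Twitch SDK OAuth via browser until logged in, then opens a TwiWorks chat feed with those tokens.
; Non-bot messages spawn or reuse a named BP_Twitch_User_Char at a random navigable point to display the text.
; Chat commands trigger jumps and dance emotes on those characters, or an explosion before the player.
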(event Custom|SetupTwitchSDK
  ;[1 1 1] Twitch SDK Setup
  (bind (_result _error) (|GetAuthState)
    (:Done
      (switch Utilities|FlowControl|Switch|SwitchonFTwitchSDKAuthStatus (.Status (Utilities|Struct|BreakTwitchSDKAuthState _result))
        (:LoggedOut
          (bind (_result_2 _error_2) (|GetAuthenticationInfo (Class|TwitchSDKBPLibrary|BuildOAuthScopes (Variables|Default|GetDefaultAuthScopes) (Variables|Default|GetCustomOAuthScopes)) :!label _label)
            (:Done
              (Development|PrintString (Utilities|String|ToString(Text) (Utilities|Text|FormatText "URI: {uri} 
User Code: {usercode}" (.Uri (Utilities|Struct|BreakTwitchSDKAuthenticationInfo _result_2)) (.UserCode (Utilities|Struct|BreakTwitchSDKAuthenticationInfo _result_2)))) true true "(R=0.000000,G=0.660000,B=1.000000,A=1.000000)" 3e+01)
              (bind _returnvalue (Class|KismetSystemLibrary|CanLaunchURL (Utilities|String|Append (.Uri (Utilities|Struct|BreakTwitchSDKAuthenticationInfo _result_2)) (.UserCode (Utilities|Struct|BreakTwitchSDKAuthenticationInfo _result_2)))))
              (if _returnvalue
                (Utilities|Platform|LaunchURL (Utilities|String|Append (.Uri (Utilities|Struct|BreakTwitchSDKAuthenticationInfo _result_2)) (.UserCode (Utilities|Struct|BreakTwitchSDKAuthenticationInfo _result_2))))
                (Utilities|FlowControl|Delay 3e+01)
                (else
                  (Utilities|FlowControl|Delay 0.2 :!label _label_2))))
            (:Error
              (Development|PrintString _error_2)
              (goto _label_2)))
          (CallFunction|SetupTwitchSDK))
        (:Loading
          (goto _label))
        (:WaitingForCode
          (goto _label))
        (:LoggedIn
          (Development|PrintString "Already Logged In")
          (Utilities|FlowControl|Delay 3.0)
          (CallFunction|SetupTwiWorks))))
    (:Error
      (Development|PrintString _error))))

(event Custom|SetupTwiWorks
  ;[1 1 1] Twiworks Setup
  (bind (_result _error) (|GetMyUserInfo)
    (:Done
      (Variables|Default|SetResult%20Channel%20Id (.channelid _result))
      (Variables|Default|SetResult%20Login%20Name (.loginname _result))
      (bind (_accesstoken _refreshtoken) (|GetAuthTokens)
        (:Done
          (Variables|Default|SetAccess%20Token _accesstoken)
          (Variables|Default|SetRefresh%20Token _refreshtoken)
          (bind _twitchchat (|RequestFeed (EventDispatchers|CreateEvent :!event Custom|OnChatMessageReceived) (EventDispatchers|CreateEvent :!event Custom|OnCheerEventReceived) (Utilities|Struct|MakeTwitchLoginCredentials (Variables|Default|GetAccess%20Token) (Variables|Default|GetResult%20Login%20Name) (Variables|Default|GetRefresh%20Token) (Variables|Default|GetResult%20Channel%20Id)) (Variables|Default|GetResult%20Login%20Name))
            (:OnSuccessfulLogin
              (Variables|Default|SetTwitch%20Chat _twitchchat)
              (CallFunction|SetAllTwitchCommands))
            (:OnFailedLogin
              (Development|PrintString "Failed to log in to twiworks" true true "(R=0.000000,G=0.660000,B=1.000000,A=1.000000)" 3e+01))
            (:OnDisconnect
              (Development|PrintString "Disconnected from TwiWorks"))))
        (:Error
          (Development|PrintString "GetAuthTokens Failed" true true "(R=0.000000,G=0.660000,B=1.000000,A=1.000000)" 3e+01))))
    (:Error
      (Development|PrintString _error true true "(R=0.000000,G=0.660000,B=1.000000,A=1.000000)" 3e+01))))

(event Custom|OnChatMessageReceived
  (params (TwitchMessage :type Twitch%20Message%20Structure))
  (bind _character (CallFunction|GetViewerCharacter (.displayname (.author TwitchMessage))))
  ;[1 1 1] On Message Received
  (Variables|Default|Setchatter%20name (.displayname (.author TwitchMessage)))
  (Variables|Default|SetIncomingMessage (Utilities|Struct|MakeS_MessageContent (.color (.author TwitchMessage)) (.displayname (.author TwitchMessage)) (.messagebody TwitchMessage)))
  (if (not (CallFunction|IsBotName (.displayname (.author TwitchMessage))))
    (if (CallFunction|DoesViewerHaveCharacter (.displayname (.author TwitchMessage)))
      (Utilities|IsValid _character
        (:Is%20Valid
          (Default|DisplayChatMessage _character (.messagebody TwitchMessage)))
        (:Is%20Not%20Valid
          (bind _randomlocation (Class|NavigationSystemV1|GetRandomLocationinNavigableRadius (Math|Vector|MakeVector 0.0 0.0 0.0) 1e+03 0 0 :!label _label))
          (bind _returnvalue (Game|SpawnActorfromClass "/Game/Twitch/BP/Character/BP_Twitch_User_Char.BP_Twitch_User_Char_C" (Math|Transform|MakeTransform _randomlocation "0, 0, 0" "1.000000,1.000000,1.000000") "Undefined" "MultiplyWithRoot" 0 (Variables|Default|Getchatter%20name) 0))
          (Utilities|Array|Add (Variables|Default|GetViewerCharNames) (Utilities|Struct|MakeS_ViewerCharacter (Variables|Default|Getchatter%20name) _returnvalue))
          (Default|DisplayChatMessage _returnvalue (.messagebody TwitchMessage))))
      (else
        (goto _label)))))

(event Custom|SetAllTwitchCommands
  ;[1 1 1] Set Up Twitch Commands
  (Utilities|FlowControl|Sequence
    (:then_0
      (|AddBoomCommand))
    (:then_1
      (|AddJumpCommand))
    (:then_2
      (|AddEmotes))))

(event Custom|CustomEvent
  (params (PointsEvent :type Twitch%20Points%20Event%20Structure))
  (Development|PrintString "points command worked"))

(event Custom|OnCheerEventReceived
  (params (TwitchCheer :type Twitch%20Cheer%20Structure))
  ;[1 1 1] On Cheer
)

(event Custom|SetupPointsEvent
  (Class|TwitchPluginBPLibrary|BindtoonPointsEvent (Variables|Default|GetTwitch%20Chat) (delegate Custom|CustomEvent)))

(event Custom|CreateViewerCharacter
  (params (InputPin :type String))
  ;[1 1 1] On Message Received
  (Variables|Default|Setchatter%20name InputPin)
  (bind _randomlocation (Class|NavigationSystemV1|GetRandomLocationinNavigableRadius (Math|Vector|MakeVector 0.0 0.0 0.0) 1e+03 0 0))
  (bind _returnvalue (Game|SpawnActorfromClass "/Game/Twitch/BP/Character/BP_Twitch_User_Char.BP_Twitch_User_Char_C" (Math|Transform|MakeTransform _randomlocation "0, 0, 0" "1.000000,1.000000,1.000000") "Undefined" "MultiplyWithRoot" 0 (Variables|Default|Getchatter%20name) 0))
  (Utilities|Array|Add (Variables|Default|GetViewerCharNames) (Utilities|Struct|MakeS_ViewerCharacter (Variables|Default|Getchatter%20name) _returnvalue))
  (Default|DisplayChatMessage _returnvalue (.messagebody (stale Custom|OnChatMessageReceived TwitchMessage))))

(event Custom|AddCustomEmote
  ;[1 1 1] Set Up Twitch Commands
  (|AddEmotes_2))

(event EventInit
  ;[1 1 1] Event Init
  (CallFunction|SetupTwitchSDK)
  (bind _returnvalue (Settings|GetGameUserSettings))
  (Class|GameUserSettings|SetScreenResolution _returnvalue (Utilities|Struct|MakeIntPoint 1280 720))
  (Class|GameUserSettings|ApplySettings _returnvalue true))

(fn IsBotName
  (params (Name :type String))
  (for _array_element (Variables|Default|GetBotNames)
    (if (Utilities|Enum|Equal(Enum) _array_element Name)
      (LocalVariables|SetmatchedBotName true)))
  (return (LocalVariables|GetmatchedBotName)))

(fn DoesViewerHaveCharacter
  (params (Name :type String))
  (bind _viewercharnames (Variables|Default|GetViewerCharNames))
  (if (> (Utilities|Array|Length _viewercharnames) 0)
    (bind _array_element (Utilities|Array|ForEachLoopwithBreak _viewercharnames :!label _label)
      (:LoopBody
        (if (Utilities|Enum|Equal(Enum) (.ViewerName (Utilities|Struct|BreakS_ViewerCharacter _array_element)) Name)
          (LocalVariables|SetHasCharacter true)
          (goto _label Break)))
      (:Completed
        (return (LocalVariables|GetHasCharacter))))
    (else
      (return (LocalVariables|GetHasCharacter)))))

(fn GetViewerCharacter
  (params (Name :type String))
  (bind _array_element (Utilities|Array|ForEachLoopwithBreak (Variables|Default|GetViewerCharNames) :!label _label)
    (:LoopBody
      (if (Utilities|Enum|Equal(Enum) (.ViewerName (Utilities|Struct|BreakS_ViewerCharacter _array_element)) Name)
        (LocalVariables|SetCharacterRef (.ViewerCharacter (Utilities|Struct|BreakS_ViewerCharacter _array_element)))
        (goto _label Break)))
    (:Completed
      (return (LocalVariables|GetCharacterRef)))))

(event Custom|OnCustomCommand
  (params (Parameters :type Array%20of%20Strings) (Sender :type Twitch%20Message%20Author%20Structure))
  (if (CallFunction|DoesViewerHaveCharacter (.displayname Sender))
    (Default|CallEmote (CallFunction|GetViewerCharacter (.displayname Sender)) "Ballet")
    (else
      (CallFunction|CreateViewerCharacter (.displayname Sender)))))

(event Custom|OnBoomCommand
  (params (Parameters :type Array%20of%20Strings) (Sender :type Twitch%20Message%20Author%20Structure))
  (bind _returnvalue (Game|Player|GetPlayerPawn 0))
  (bind _returnvalue_2 (Transformation|GetActorLocation _returnvalue))
  (bind _returnvalue_3 (Transformation|GetActorForwardVector _returnvalue))
  (bind _returnvalue_4 (* _returnvalue_3 1.5e+02))
  (bind _returnvalue_5 (+ _returnvalue_2 _returnvalue_4))
  (Effects|SpawnEmitteratLocation "/Game/StarterContent/Particles/P_Explosion.P_Explosion" _returnvalue_5 "0, 0, 0" "2.000000,2.000000,2.000000")
  (Audio|PlaySoundatLocation "/Game/Twitch/Audio/WAV_Explosion.WAV_Explosion" _returnvalue_5 "0, 0, 0" 2.0 1.0 0.0 0 0 0 0))

(event Custom|OnJumpCommand
  (params (Parameters :type Array%20of%20Strings) (Sender :type Twitch%20Message%20Author%20Structure))
  (if (CallFunction|DoesViewerHaveCharacter (.displayname Sender))
    (Character|Jump (CallFunction|GetViewerCharacter (.displayname Sender)))
    (else
      (CallFunction|CreateViewerCharacter (.displayname Sender)))))

(event Custom|OnBalletCommand
  (params (Parameters :type Array%20of%20Strings) (Sender :type Twitch%20Message%20Author%20Structure))
  (if (CallFunction|DoesViewerHaveCharacter (.displayname Sender))
    (Default|CallEmote (CallFunction|GetViewerCharacter (.displayname Sender)) "Ballet")
    (else
      (CallFunction|CreateViewerCharacter (.displayname Sender)))))

(event Custom|OnChickenCommand
  (params (Parameters :type Array%20of%20Strings) (Sender :type Twitch%20Message%20Author%20Structure))
  (if (CallFunction|DoesViewerHaveCharacter (.displayname Sender))
    (Default|CallEmote (CallFunction|GetViewerCharacter (.displayname Sender)) "Chicken")
    (else
      (CallFunction|CreateViewerCharacter (.displayname Sender)))))

(event Custom|OnBreakdanceCommand
  (params (Parameters :type Array%20of%20Strings) (Sender :type Twitch%20Message%20Author%20Structure))
  (if (CallFunction|DoesViewerHaveCharacter (.displayname Sender))
    (Default|CallEmote (CallFunction|GetViewerCharacter (.displayname Sender)) "Breakdance")
    (else
      (CallFunction|CreateViewerCharacter (.displayname Sender)))))

(event Custom|OnWaveCommand
  (params (Parameters :type Array%20of%20Strings) (Sender :type Twitch%20Message%20Author%20Structure))
  (if (CallFunction|DoesViewerHaveCharacter (.displayname Sender))
    (Default|CallEmote (CallFunction|GetViewerCharacter (.displayname Sender)) "Wave")
    (else
      (CallFunction|CreateViewerCharacter (.displayname Sender)))))

(event Custom|OnThrillerCommand
  (params (Parameters :type Array%20of%20Strings) (Sender :type Twitch%20Message%20Author%20Structure))
  (if (CallFunction|DoesViewerHaveCharacter (.displayname Sender))
    (Default|CallEmote (CallFunction|GetViewerCharacter (.displayname Sender)) "Thriller")
    (else
      (CallFunction|CreateViewerCharacter (.displayname Sender)))))