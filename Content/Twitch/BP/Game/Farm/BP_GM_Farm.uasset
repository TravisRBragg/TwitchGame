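; Game mode for the Farm level that links Twitch chat, predictions, polls and raids to gameplay.
; BeginPlay retries until the game instance's TwitchChat is valid, then resets custom rewards and binds raids, which spawn physics balls before the player.
; Callable events run predictions and polls through re-armed wait loops, printing the poll winner.
; The "Spawn Balls" reward handler is unwired; setup and Destroyed call ReplaceCustomRewards without a list.
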(event Custom|CallCreatePrediction
  (params (title :type String) (Outcomes :type Array%20of%20Strings) (duration :type Integer))
  ;[1 1 1] Prediction Logic
  (bind (_result _error) (|Prediction title Outcomes duration)
    (:Done
      (Variables|Default|SetPredictionID (.Id (Utilities|Struct|BreakTwitchSDKPredictionInfo _result)))
      (Variables|Default|SetBroadcasterId (.BroadcasterId (Utilities|Struct|BreakTwitchSDKPredictionInfo _result)))
      (bind (_result_2 _error_2) (|WaitforPredictionUpdate (Variables|Default|GetPredictionID) :!label _label)
        (:Done
          (switch Utilities|FlowControl|Switch|SwitchonFTwitchSDKPredictionStatus (.Status (Utilities|Struct|BreakTwitchSDKPredictionInfo _result_2))
            (:Active
              (goto _label))
            (:Locked
              (Development|PrintString "Locked")
              (Variables|Default|SetOutcomesStructArray (.Outcomes (Utilities|Struct|BreakTwitchSDKPredictionInfo _result_2))))
            (:Resolved
              (CallFunction|CallCancelPrediction :!label _label_2))
            (:Canceled
              (goto _label_2))))
        (:Error
          (Development|PrintString _error_2))))
    (:Error
      (Development|PrintString _error))))

(event Custom|CallCancelPrediction
  (bind _predictionid (Variables|Default|GetPredictionID))
  ;[1 1 1] Prediction Logic
  (|EndPrediction (Variables|Default|GetBroadcasterId) _predictionid "Canceled"
    (:Done
      _)
    (:Error
      _))
  (|UnsubscribefromPrediction _predictionid))

(event Custom|CallResolvePrediction
  (params (OutcomeTitle :type String))
  ;[1 1 1] Prediction Logic
  (for _array_element (Variables|Default|GetOutcomesStructArray)
    (if (Utilities|Enum|Equal(Enum) (.Title (Utilities|Struct|BreakTwitchSDKPredictionOutcome _array_element)) OutcomeTitle)
      (Variables|Default|SetWinningStruct _array_element)))
  (bind (_result _error) (|EndPrediction (Variables|Default|GetBroadcasterId) (Variables|Default|GetPredictionID) "Resolved" (.Id (Utilities|Struct|BreakTwitchSDKPredictionOutcome (Variables|Default|GetWinningStruct))))
    (:Done
      (switch Utilities|FlowControl|Switch|SwitchonFTwitchSDKPredictionStatus (.Status (Utilities|Struct|BreakTwitchSDKPredictionInfo _result))
        (:Active
          _)
        (:Locked
          _)
        (:Resolved
          _)
        (:Canceled
          _)))
    (:Error
      (Development|PrintString _error)))
  (CallFunction|CallCancelPrediction))

(event Custom|CallCreatePoll
  (params (title :type String) (Choices :type Array%20of%20Strings) (duration :type Integer64) (bitsVotingEnabled :type Boolean) (bitsPerVote :type Integer) (channelPointsVotingEnabled :type Boolean) (channelPointsPerVote :type Integer))
  ;[1 1 1] Poll Logic
  (bind (_result _error) (|Poll title Choices duration bitsVotingEnabled bitsPerVote channelPointsVotingEnabled channelPointsPerVote)
    (:Done
      (Variables|Default|SetPoll_ID (.Id (Utilities|Struct|BreakTwitchSDKPollInfo _result)))
      (Variables|Default|SetBroadcasterId (.BroadcasterId (Utilities|Struct|BreakTwitchSDKPollInfo _result)))
      (Variables|Default|SetPollVoteAmount 0)
      (bind (_result_2 _error_2) (|WaitforPollUpdate (Variables|Default|GetPoll_ID) :!label _label)
        (:Done
          (switch Utilities|FlowControl|Switch|SwitchonFTwitchSDKPollStatus (.Status (Utilities|Struct|BreakTwitchSDKPollInfo _result_2))
            (:Active
              (goto _label))
            (:Completed
              (for _array_element (.Choices (Utilities|Struct|BreakTwitchSDKPollInfo _result_2))
                (if (> (.Votes (Utilities|Struct|BreakTwitchSDKPollChoiceInfo _array_element)) (Variables|Default|GetPollVoteAmount))
                  (Variables|Default|SetPollVote_Text (.Title (Utilities|Struct|BreakTwitchSDKPollChoiceInfo _array_element)))
                  (Variables|Default|SetPollVoteAmount (.Votes (Utilities|Struct|BreakTwitchSDKPollChoiceInfo _array_element)))))
              (Development|PrintString (Utilities|String|ToString(Text) (Utilities|Text|FormatText "The winning vote was {winner} with {numvotes} total votes" (Variables|Default|GetPollVote_Text) (Variables|Default|GetPollVoteAmount))) true true "(R=0.000000,G=0.660000,B=1.000000,A=1.000000)" 3e+01)
              (|UnsubscribefromPoll (Variables|Default|GetPoll_ID)))
            (:Terminated
              (|UnsubscribefromPoll (Variables|Default|GetPoll_ID) :!label _label_2))))
        (:Error
          (Development|PrintString _error_2)
          (goto _label_2))))
    (:Error
      (Development|PrintString _error)
      (goto _label_2))))

(event Custom|SetUpCustomRewards
  (|ReplaceCustomRewards))

(event Custom|CallWaitForRaid
  ;[1 1 1] Raid Logic
  (Class|TwitchPluginBPLibrary|BindtoonRaid (Variables|Default|GetTwitch%20Chat) (delegate Custom|OnRaid)))

(event Custom|OnRaid
  (params (RaidEvent :type Twitch%20Raid%20Event%20Structure))
  ;[1 1 1] Raid Logic
  (for _index (range 0 20)
    (Game|SpawnActorfromClass "/Game/Twitch/BP/Test/BP_PhysicsBall.BP_PhysicsBall_C" (Math|Transform|MakeTransform (CallFunction|GetRandomSpawnPointsFrontOfPawn) "0, 0, 0" "1.000000,1.000000,1.000000") "Undefined" "MultiplyWithRoot" 0 0)))

(event EventDestroyed
  (|ReplaceCustomRewards))

(event EventBeginPlay
  ;[1 1 1] Begin Play / Call Other Logic
  (bind _asbp_twitch_game_instance (Utilities|Casting|CastToBP_Twitch_Game_Instance (Game|GetGameInstance)))
  (bind _output_get (Variables|Default|SetAs%20BP%20Twitch%20Game%20Instance _asbp_twitch_game_instance))
  (bind _twitch_chat (Variables|/Game/Twitch/BP/Game/BP_Twitch_Game_Instance.BP_Twitch_Game_Instance_C|GetTwitch%20Chat _output_get :!label _label)
    (:then
      (Variables|Default|SetTwitch%20Chat _twitch_chat)
      (CallFunction|SetUpCustomRewards)
      (CallFunction|CallWaitforRaid))
    (:else
      (Utilities|FlowControl|Delay 0.2)
      (goto _label))))

(fn ConstructionScript)

(fn GetRandomSpawnPointsFrontOfPawn
  (bind _returnvalue (Game|Player|GetPlayerPawn 0))
  (return (+ (+ (Transformation|GetActorLocation _returnvalue) (* (Transformation|GetActorForwardVector _returnvalue) (Math|Random|RandomFloatinRange 5e+02 7.5e+02))) (* (Transformation|GetActorRightVector _returnvalue) (Math|Random|RandomFloatinRange -5e+02 5e+02)))))