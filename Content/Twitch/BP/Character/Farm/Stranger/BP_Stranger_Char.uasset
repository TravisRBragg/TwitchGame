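; Stranger NPC for weed sales that may turn out to be undercover, with a random mesh picked at construction.
; On spawn it walks a short offset and becomes interactable, or destroys itself if the move fails.
; Interact plays a sale montage; TriggerArrest loops a gun-pointing montage, and each notifies the interacting actor before self-destructing.
; The undercover check is a weighted random roll on every call, not stored state.
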(event EventBeginPlay
  (AI|AIMoveTo self (+ (Transformation|GetActorLocation) "0.000000,500.000000,0.000000") 0 2e+01 false
    (:OnSuccess
      (Variables|Default|SetCan%20Interact? true))
    (:OnFail
      (Utilities|FlowControl|Delay 0.2)
      (Actor|DestroyActor))))

(event EventInteract
  (params (InteractingActor :type Actor%20Object%20Reference))
  (Variables|Default|SetCan%20Interact? false)
  (Animation|Montage|PlayMontage (Variables|Character|GetMesh) "/Game/Characters/Mixamo/Stranger/Anims/AM_SellWeed.AM_SellWeed"
    (:OnCompleted
      (Class|BPIInteractable|SuccessfulSale(Message) InteractingActor)
      (Actor|DestroyActor))))

(event EventTriggerArrest
  (params (InteractingActor :type Actor%20Object%20Reference))
  (Variables|Default|SetCan%20Interact? false)
  (Animation|Montage|PlayMontage (Variables|Character|GetMesh) "/Game/Characters/Mixamo/Stranger/Anims/AM_PointGun.AM_PointGun" :!label _label
    (:then
      (Utilities|FlowControl|DoOnce false
        (:Completed
          (Utilities|FlowControl|Delay 2.0)
          (Class|BPIInteractable|TriggerArrest(Message) InteractingActor)
          (Actor|DestroyActor))))
    (:OnBlendOut
      (Utilities|FlowControl|Delay (Utilities|Time|GetWorldDeltaSeconds))
      (goto _label))))

(fn ConstructionScript
  (Components|SkeletalMesh|SetSkeletalMeshAsset (Variables|Character|GetMesh) (.OutItem (Utilities|Array|Random (Variables|Default|GetMeshes)))))

(fn GetCurrentState
  (return "NewEnumerator0"))

(fn CanbeInteractedWith?
  (return (Variables|Default|GetCan%20Interact?)))

(fn IsUndercover?
  (return (Math|Random|RandomBoolwithWeight 0.2)))