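; Character representing a Twitch viewer, with a name label, tinted materials, emotes, timed chat message widget and crop, cash, XP and level stats.
; It wanders to random navigable points while idle; emotes and farm tasks hold off new wandering.
; WorkOnCrop walks it to a plot, plays the plant, water or harvest montage, then notifies the plot and game instance and awards XP, plus crops on harvest.
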(event Custom|DisplayChatMessage
  (params (Message :type String) (MessageColor :type Linear%20Color%20Structure))
  (bind _widget (Variables|Default|GetWidget))
  (bind _messagewidget (Variables|Default|GetMessageWidget)
    (:then
      (Widget|RemovefromParent _messagewidget))
    (:else
      _))
  (bind _returnvalue (UserInterface|CreateWidget "/Game/Twitch/UI/Character/W_Viewer_Message.W_Viewer_Message_C" 0 Message MessageColor))
  (bind _output_get (Variables|Default|SetMessageWidget _returnvalue))
  (UserInterface|SetWidget _widget _output_get)
  (Utilities|FlowControl|Delay 5.0)
  (UserInterface|SetWidget _widget 0))

(event Custom|Start%20Moving
  (if (or (Variables|Default|GetDoingTask) (Variables|Default|GetisEmoting))
    _
    (else
      (bind _randomlocation (Class|NavigationSystemV1|GetRandomLocationinNavigableRadius (Math|Vector|MakeVector 0.0 0.0 0.0) 1e+03 0 0))
      (AI|AIMoveTo self _randomlocation 0 5e+01 false
        (:OnSuccess
          _)
        (:OnFail
          _))))
  (Utilities|FlowControl|Delay 5.0)
  (CallFunction|StartMoving))

(event Custom|CallEmote
  (params (AnimMontage :type Anim%20Montage%20Object%20Reference))
  (if (not (Variables|Default|GetDoingTask))
    (Variables|Default|SetisEmoting true)
    (Components|Movement|StopMovementImmediately (Variables|Character|GetCharacterMovement))
    (bind _returnvalue (Animation|PlayAnimMontage AnimMontage 1.0 "None"))
    (Utilities|FlowControl|Delay _returnvalue)
    (Variables|Default|SetisEmoting false)))

(event Custom|WorkOnCrop
  (params (TargetPlot :type Actor%20Object%20Reference) (Task :type E_CropJob%20Enum :default "NewEnumerator0"))
  (bind _self self)
  (bind _mesh (Variables|Character|GetMesh))
  (bind _gameinst (Variables|Default|GetGameInst))
  (Variables|Default|SetTarget%20Plot TargetPlot)
  (Variables|Default|SetCurrentTast Task)
  (Variables|Default|SetDoingTask true)
  (Variables|Default|SetisEmoting false)
  (AI|AIMoveTo self "0, 0, 0" (Variables|Default|GetTarget%20Plot) 5e+01 false
    (:OnSuccess
      (Transformation|SetActorRotation (Math|Rotator|MakeRotator 0.0 0.0 (.yaw (Math|Rotator|FindLookatRotation (Transformation|GetActorLocation) (Transformation|GetActorLocation (Variables|Default|GetTarget%20Plot))))))
      (switch Utilities|FlowControl|Switch|SwitchonE_CropJob (Variables|Default|GetCurrentTast)
        (:NewEnumerator0
          (Animation|Montage|PlayMontage _mesh "/Game/Twitch/Anims/AM_Dig_And_Plant_Seeds.AM_Dig_And_Plant_Seeds"
            (:OnBlendOut
              (Class|BPICrop|PlantSeed(Message) (Variables|Default|GetTarget%20Plot)))))
        (:NewEnumerator1
          (Animation|Montage|PlayMontage _mesh "/Game/Twitch/Anims/AM_Watering.AM_Watering"
            (:OnBlendOut
              (Class|BPICrop|WaterCrop(Message) (Variables|Default|GetTarget%20Plot)))))
        (:NewEnumerator2
          (Animation|Montage|PlayMontage _mesh "/Game/Twitch/Anims/AM_Pick_Fruit.AM_Pick_Fruit"
            (:OnBlendOut
              (Class|BPICrop|HarvestPlant(Message) (Variables|Default|GetTarget%20Plot))))))
      (Utilities|FlowControl|Delay 1.0)
      (Variables|Default|SetDoingTask false)
      (switch Utilities|FlowControl|Switch|SwitchonE_CropJob (Variables|Default|GetCurrentTast)
        (:NewEnumerator0
          (Default|CallSeedCrop _gameinst _self)
          (CallFunction|IncrementXP 10))
        (:NewEnumerator1
          (Default|CallWaterCrop _gameinst _self)
          (CallFunction|IncrementXP 10))
        (:NewEnumerator2
          (Default|CallHarvestCrop _gameinst _self)
          (CallFunction|IncrementCrops (Math|Random|RandomIntegerinRange 1 15))
          (CallFunction|IncrementXP 15))))
    (:OnFail
      (Development|PrintString "Failed to nav")
      (Class|BPICrop|SetIsInteracted(Message) (Variables|Default|GetTarget%20Plot) false))))

(event EventBeginPlay
  (Rendering|Components|TextRender|SetText (Variables|Default|GetTextRender) (Utilities|Text|ToText(String) (Variables|Default|GetPlayerName)))
  (CallFunction|StartMoving)
  (bind _asbp_twitch_game_instance (Utilities|Casting|CastToBP_Twitch_Game_Instance (Game|GetGameInstance)))
  (Variables|Default|SetGameInst _asbp_twitch_game_instance))

(event Collision|EventActorBeginOverlap
  (params (OtherActor :type Actor%20Object%20Reference)))

(event EventTick
  (params (DeltaSeconds :type Float%20%28single-precision%29))
  (bind _returnvalue (Transformation|GetActorLocation))
  (bind _returnvalue_2 (Game|GetPlayerCameraManager 0))
  (bind _returnvalue_3 (Transformation|GetActorLocation _returnvalue_2))
  (bind _returnvalue_4 (Math|Rotator|FindLookatRotation _returnvalue _returnvalue_3))
  (Transformation|SetWorldRotation (Variables|Default|GetTextRender) (Math|Rotator|MakeRotator (.roll _returnvalue_4) (.pitch _returnvalue_4) 1.8e+02) false false))

(fn ConstructionScript
  (bind _mesh (Variables|Character|GetMesh))
  (bind _returnvalue (Rendering|Material|CreateDynamicMaterialInstance _mesh 0 0 "None" :!class /Script/Engine.PrimitiveComponent))
  (Variables|Default|SetDynMat1 _returnvalue)
  (bind _returnvalue_2 (Rendering|Material|CreateDynamicMaterialInstance _mesh 1 0 "None" :!class /Script/Engine.PrimitiveComponent))
  (Variables|Default|SetDynMat2 _returnvalue_2)
  (Rendering|Material|SetVectorParameterValue (Variables|Default|GetDynMat1) "Tint" (Variables|Default|GetCharColor) :!class /Script/Engine.MaterialInstanceDynamic))

(fn OnRepPlayerName)

(fn GetStats
  (return (Utilities|Struct|MakeS_TwitchViewerStats (Variables|Default|GetPlayerName) (Variables|Default|GetNumHarvestCrops) (Variables|Default|GetCash) (Variables|Default|GetXP) (Variables|Default|GetLevel))))

(fn IncrementXP
  (params (Added%20XP :type Integer))
  (bind _output_get (Variables|Default|SetXP (+ (Variables|Default|GetXP) Added%20XP)))
  (if (>= _output_get (* (Variables|Default|GetLevel) 20))
    (Variables|Default|SetXP (- (Variables|Default|GetXP) (* (Variables|Default|GetLevel) 20)))
    (CallFunction|IncrementLevel)))

(fn IncrementCrops
  (params (Added%20Crops :type Integer))
  (Variables|Default|SetNumHarvestCrops (+ Added%20Crops (Variables|Default|GetNumHarvestCrops))))

(fn IncrementCash
  (params (Added%20Cash :type Integer))
  (Variables|Default|SetCash (+ Added%20Cash (Variables|Default|GetCash))))

(fn IncrementLevel
  (Math|Integer|IncrementInt (Variables|Default|GetLevel)))

(fn GetCurrentState
  (return "NewEnumerator0"))